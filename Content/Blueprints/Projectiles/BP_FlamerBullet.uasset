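; BP_FlamerBullet is a flamethrower projectile that damages player bots.
; On BeginPlay it stores its location and spawns a one-shot flame particle effect there.
; Each tick on the server, it line-traces between its current and previous locations, ignoring the instigator, with debug drawing left on.
; A hit on BP_PlayerBot passes damage, bone and location to that bot, and any hit destroys the projectile.
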(event `self.ReceiveBeginPlay`
  (set `self.lastLocation` (`SceneComponent.K2_GetComponentLocation` (`self.DefaultSceneRoot`)))
  (`GameplayStatics.SpawnEmitterAtLocation` "/Game/Realistic_Starter_VFX_Pack_Vol2/Particles/Fire/P_flamethrowerOneShot.P_flamethrowerOneShot" (`self.K2_GetActorLocation`) (`self.K2_GetActorRotation`)))

(event `self.ReceiveTick`
  (params (DeltaSeconds :type "Float (single-precision)"))
  (bind _returnvalue (`SceneComponent.K2_GetComponentLocation` (`self.DefaultSceneRoot`)))
  (if (`KismetSystemLibrary.IsServer`)
    (bind (_outhit _returnvalue_2) (`KismetSystemLibrary.LineTraceSingleForObjects` _returnvalue (`self.lastLocation`) (`|MakeArray` "ObjectTypeQuery3" "ObjectTypeQuery1" :!type "EObjectTypeQuery Enum") false (`|MakeArray` (`self.GetInstigator`) :!type "Actor Object Reference") "ForDuration"))
    (set `self.lastLocation` _returnvalue)
    (if _returnvalue_2
      (bind (_bblockinghit _binitialoverlap _time _distance _location _impactpoint _normal _impactnormal _physmat _hitactor _hitcomponent _hitbonename) (`GameplayStatics.BreakHitResult` _outhit))
      (bind _asbp_player_bot (cast `/Game/Blueprints/PlayerBot/BP_PlayerBot` _hitactor)
        (:`then`
          (`/Game/Blueprints/PlayerBot/BP_PlayerBot.Damage` _asbp_player_bot _hitbonename (`self.Damage`) _location)
          (`self.K2_DestroyActor`))
        (:`CastFailed`
          (`self.K2_DestroyActor`))))))

(fn `UserConstructionScript`)