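; BP_WeaponItem is a weapon item that displays a skeletal mesh from its ItemStat and can be picked up.
; On BeginPlay, a valid ItemStat and mesh set WeaponMesh and seed ActiveData from StartingHealth.
; SetItemData replaces the stat, mesh and active data, so an item can carry existing state.
; PickUpItem only returns ItemStat and ActiveData, leaving any removal from the world to other code.
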(event `self.ReceiveBeginPlay`
  (bind _itemstat (`self.ItemStat`)
    (:`then`
      (bind _itemmesh (`/Game/Blueprints/Items/Weapons/BP_WeaponData.ItemMesh` _itemstat)
        (:`then`
          (`SkeletalMeshComponent.SetSkeletalMeshAsset` (`self.WeaponMesh`) _itemmesh)
          (set `self.ActiveData` (make `/Game/Blueprints/Items/Weapons/ActiveWeaponData` (`/Game/Blueprints/Items/Weapons/BP_WeaponData.StartingHealth` _itemstat))))
        (:`else`)))
    (:`else`)))

(fn `PickUpItem`
  (returns (Item :type "/Game/Blueprints/Items/Weapons/BP_WeaponData Object Reference") (ActiveItemData :type "/Game/Blueprints/Items/Weapons/ActiveWeaponData Structure"))
  (return (`self.ItemStat`) (`self.ActiveData`)))

(fn `Set Item Data`
  (params (WeaponItemStat :type "/Game/Blueprints/Items/Weapons/BP_WeaponData Object Reference") (ActiveWeaponData :type "/Game/Blueprints/Items/Weapons/ActiveWeaponData Structure"))
  (bind _output_get (set `self.ItemStat` WeaponItemStat))
  (`SkeletalMeshComponent.SetSkeletalMeshAsset` (`self.WeaponMesh`) (`/Game/Blueprints/Items/Weapons/BP_WeaponData.ItemMesh` _output_get))
  (set `self.ActiveData` ActiveWeaponData))

(fn `UserConstructionScript`)